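; Player ship pawn driven by movement axis inputs and turned toward the mouse cursor.
; All four axes feed FloatingPawnMovement, each applying its value equally to world X and Y, so every input moves along the same diagonal.
; BeginPlay shows the cursor; Tick traces under it on Visibility and slowly interpolates Scene1's relative rotation toward a look-at of the hit point.
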(event EventBeginPlay
  (bind _returnvalue (Class|InputDeviceLibrary|GetPlayerControllerfromInputDevice))
  (Variables|/Script/Engine.PlayerController|SetbShowMouseCursor _returnvalue true))

(event Collision|EventActorBeginOverlap
  (params (OtherActor :type Actor%20Object%20Reference)))

(event EventTick
  (params (DeltaSeconds :type Float%20%28single-precision%29))
  (bind _returnvalue (Class|InputDeviceLibrary|GetPlayerControllerfromInputDevice))
  (Transformation|SetRelativeRotation (Variables|Default|GetScene1) (Math|Interpolation|RInterpTo (Variables|/Script/Engine.SceneComponent|GetRelativeRotation (Variables|Default|GetScene1)) (Math|Rotator|FindLookatRotation (Transformation|GetActorLocation) (.Location (Collision|BreakHitResult (.HitResult (Game|Player|GetHitResultUnderCursorbyChannel _returnvalue "TraceTypeQuery1" true))))) DeltaSeconds 0.2) false false))

(event Input|AxisEvents|InputAxisMoveUp
  (params (AxisValue :type Float%20%28single-precision%29))
  (Class|PawnMovementComponent|AddInputVector (Variables|Default|GetFloatingPawnMovement) (Math|Vector|MakeVector AxisValue (stale Input|AxisEvents|InputAxisMoveRight AxisValue) 0.0) false))

(event Input|AxisEvents|InputAxisMoveRight
  (params (AxisValue :type Float%20%28single-precision%29))
  (Class|PawnMovementComponent|AddInputVector (Variables|Default|GetFloatingPawnMovement) (Math|Vector|MakeVector (stale Input|AxisEvents|InputAxisMoveUp AxisValue) AxisValue 0.0) false))

(event Input|AxisEvents|InputAxisMoveLeft
  (params (AxisValue :type Float%20%28single-precision%29))
  (Class|PawnMovementComponent|AddInputVector (Variables|Default|GetFloatingPawnMovement) (Math|Vector|MakeVector (stale Input|AxisEvents|InputAxisMoveDown AxisValue) AxisValue 0.0) false))

(event Input|AxisEvents|InputAxisMoveDown
  (params (AxisValue :type Float%20%28single-precision%29))
  (Class|PawnMovementComponent|AddInputVector (Variables|Default|GetFloatingPawnMovement) (Math|Vector|MakeVector AxisValue (stale Input|AxisEvents|InputAxisMoveLeft AxisValue) 0.0) false))

(fn ConstructionScript)